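; Weapon spawner actor that periodically drops weapon pickups into the level.
; On BeginPlay it starts two looping timers, one spawning a BP_Shotgun and a slower one spawning a BP_Minigun.
; Each spawn picks a random point inside the SpawnVolume box, with no cap or cleanup of earlier spawns.
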(event Custom|Shotgun
  (bind _spawn_volume (Variables|Default|GetSpawn%20Volume))
  (Game|SpawnActorfromClass "/Game/Blueprints/Player/BP_Shotgun.BP_Shotgun_C" (Math|Conversions|ToTransform(Vector) (Math|Random|RandomPointinBoundingBox (Transformation|GetWorldLocation _spawn_volume) (Components|Box|GetScaledBoxExtent _spawn_volume))) "Undefined" 0 0))

(event Custom|WeaponSpawn
  (bind _spawn_volume (Variables|Default|GetSpawn%20Volume))
  (Game|SpawnActorfromClass "/Game/Blueprints/Player/BP_Minigun.BP_Minigun_C" (Math|Conversions|ToTransform(Vector) (Math|Random|RandomPointinBoundingBox (Transformation|GetWorldLocation _spawn_volume) (Components|Box|GetScaledBoxExtent _spawn_volume))) "Undefined" 0 0))

(event EventBeginPlay
  (Utilities|Time|SetTimerbyEvent (delegate Custom|WeaponSpawn) 47.0 true)
  (Utilities|Time|SetTimerbyEvent (delegate Custom|Shotgun) 3e+01 true))

(fn ConstructionScript)