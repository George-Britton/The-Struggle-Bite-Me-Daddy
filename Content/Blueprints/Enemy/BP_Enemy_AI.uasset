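; Enemy actor for a twin-stick game that chases the player, damages them on contact and destroys itself when its health runs out.
; Looping timers re-issue AI MoveTo at the player and, less often, show one of four directional sprites by comparing X/Y positions.
; Box overlap calls TakeDamage and PlayerBlink on TwinStickPawn, while Tick polls EnemyHealth.
; BeginPlay increments a local spawn counter, but its GameInstance update is disconnected.
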(event OnComponentBeginOverlap(Box)
  (params (OverlappedComponent :type Primitive%20Component%20Object%20Reference) (OtherActor :type Actor%20Object%20Reference) (OtherComp :type Primitive%20Component%20Object%20Reference) (OtherBodyIndex :type Integer) (bFromSweep :type Boolean) (SweepResult :type Hit%20Result%20Structure%20%28by%20ref%29))
  ;[1 1 1] HP
  (bind _astwin_stick_pawn (Utilities|Casting|CastToTwinStickPawn OtherActor))
  (Default|TakeDamage _astwin_stick_pawn)
  (Default|PlayerBlink _astwin_stick_pawn))

(event Custom|EnemyFollowPlayer
  ;[1 1 1] AI Moves to Player Upon Play
  (AI|AIMoveTo self "0, 0, 0" (Game|Player|GetPlayerPawn 0) 0.0 false))

(event Custom|CheckSpritePosition
  (bind _returnvalue (Game|Player|GetPlayerPawn 0))
  (bind _returnvalue_2 (Transformation|GetActorLocation))
  (bind _returnvalue_3 (Game|Player|GetPlayerPawn 0))
  (bind _returnvalue_4 (Transformation|GetActorLocation))
  (bind _spriter (Variables|Default|GetSpriteR))
  (bind _returnvalue_5 (Transformation|GetActorLocation _returnvalue))
  (bind _returnvalue_6 (Transformation|GetActorLocation _returnvalue_3))
  (if (> (- (.y _returnvalue_5) (.y _returnvalue_2)) (- (.x _returnvalue_6) (.x _returnvalue_4)))
    ;[1 1 1] Sets Sprite
    (Math|Float|CompareFloat (.x _returnvalue_6) (.x _returnvalue_4)
      (:>
        (Development|SetHiddeninGame (Variables|Default|GetSpriteL) false false)
        (Development|SetHiddeninGame _spriter true false))
      (:<
        (Development|SetHiddeninGame (Variables|Default|GetSpriteF) false false)
        (Development|SetHiddeninGame _spriter true false)))
    (else
      ;[1 1 1] Sets Sprite
      (Math|Float|CompareFloat (.y _returnvalue_5) (.y _returnvalue_2)
        (:>
          (Development|SetHiddeninGame (Variables|Default|GetSpriteB) false false)
          (Development|SetHiddeninGame (Variables|Default|GetSpriteR) true false))
        (:<
          (Development|SetHiddeninGame (Variables|Default|GetSpriteR) false false)
          (Development|SetHiddeninGame (Variables|Default|GetSpriteL) true false))))))

(event EventTick
  (params (DeltaSeconds :type Float%20%28single-precision%29))
  (Utilities|FlowControl|Sequence
    (:then_0
      ;[1 1 1] Enemy HP
      (if (<= (Variables|Default|GetEnemyHealth) 0)
        (Actor|DestroyActor)))))

(event EventBeginPlay
  ;[1 1 1] AI Moves to Player Upon Play
  (Utilities|Time|SetTimerbyFunctionName 0 "CheckSpritePosition" 1.0 true)
  (Variables|Default|SetEnemySpawned (+ (Variables|Default|GetEnemySpawned) 1))
  (Utilities|Time|SetTimerbyEvent (delegate Custom|EnemyFollowPlayer) 0.3 true)
  (AI|AIMoveTo self "0, 0, 0" (Game|Player|GetPlayerPawn 0) 0.0 false))

(fn ConstructionScript)