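; Bon Jovi enemy that chases and damages the twin-stick player, and also stages the encounter leading into the JonDate level.
; FightStart cuts its health in proportion to the GameInstance's JonAffScore, then re-issues AIMoveTo toward the player on a looping timer.
; Box overlap damages and blinks the player, while Tick teleports it away and destroys it at zero health.
; StartEncounter slides it to LocationB by Timeline, then opens JonDate after a delay.
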(event OnComponentBeginOverlap(Box)
  (params (OverlappedComponent :type Primitive%20Component%20Object%20Reference) (OtherActor :type Actor%20Object%20Reference) (OtherComp :type Primitive%20Component%20Object%20Reference) (OtherBodyIndex :type Integer) (bFromSweep :type Boolean) (SweepResult :type Hit%20Result%20Structure%20%28by%20ref%29))
  ;[1 1 1] Player HP
  (bind _astwin_stick_pawn (Utilities|Casting|CastToTwinStickPawn OtherActor))
  (Default|TakeDamage _astwin_stick_pawn)
  (Default|PlayerBlink _astwin_stick_pawn))

(event Custom|EnemyFollowPlayer
  ;[1 1 1] AI Moves to Player Upon Play
  (AI|AIMoveTo self "0, 0, 0" (Game|Player|GetPlayerPawn 0) 0.0 false))

(event Custom|StartEncounter
  ;[1 1 1] StartsEncounter
  (Variables|Default|SetLocationA (Transformation|GetActorLocation))
  (bind _traveltime (Timeline|Timeline_0 Play)
    (:Update
      (Transformation|SetActorLocation (Math|Vector|Lerp(Vector) (Variables|Default|GetLocationA) (Variables|Default|GetLocationB) _traveltime) false false)
      (Utilities|FlowControl|Delay 6.0)
      (Game|OpenLevel(byName) "JonDate"))))

(event Custom|FightStart
  ;[1 1 1] Lowers HP Based on Higher Score
  (bind _asbp_game_instance (Utilities|Casting|CastToBP_GameInstance (Game|GetGameInstance)))
  (Variables|Default|SetEnemyHealth (- (Variables|Default|GetEnemyHealth) (Math|Float|Truncate (* (Variables|Default|GetEnemyHealth) (/ (Math|Conversions|ToFloat(Integer) (Variables|/Game/Blueprints/BP_GameInstance.BP_GameInstance_C|GetJonAffScore _asbp_game_instance)) 1e+01)))))
  ;[1 1 1] AI Moves to Player Upon Play
  (Utilities|Time|SetTimerbyEvent (delegate Custom|EnemyFollowPlayer) 0.3 true)
  (AI|AIMoveTo self "0, 0, 0" (Game|Player|GetPlayerPawn 0) 0.0 false))

(event EventTick
  (params (DeltaSeconds :type Float%20%28single-precision%29))
  ;[1 1 1] Enemy HP
  (if (<= (Variables|Default|GetEnemyHealth) 0)
    (Variables|Default|SetDead true)
    (Transformation|SetActorLocation "5000.000000,5000.000000,5000.000000" false true)
    (Utilities|FlowControl|Delay 0.2)
    (Actor|DestroyActor)))

(fn ConstructionScript)