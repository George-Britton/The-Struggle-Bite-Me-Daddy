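; BP_EnemySpawner spawns BP_Enemy_AI enemies at random points inside its SpawnVolume box.
; The EnemySpawn event starts a looping timer at the GameInstance's spawn rate, with each firing spawning one enemy and incrementing a counter.
; Tick compares that counter to the GameInstance's spawn limit, then resets it and re-sets the timer as non-looping, leaving one final spawn pending.
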(event Custom|EnemySpawn
  ;[1 1 1] Spawns Enemies
  (Variables|Default|SetMultiple%20Spawns true)
  (bind _asbp_game_instance (Utilities|Casting|CastToBP_GameInstance (Game|GetGameInstance)))
  (Utilities|Time|SetTimerbyEvent (delegate Custom|Numberofenemiesspawned) (Variables|/Game/Blueprints/BP_GameInstance.BP_GameInstance_C|GetEnemy%20Spawn%20Rate _asbp_game_instance) (Variables|Default|GetMultiple%20Spawns)))

(event Custom|Numberofenemiesspawned
  (bind _spawn_volume (Variables|Default|GetSpawn%20Volume))
  ;[1 1 1] Spawns Enemies
  (Variables|Default|SetEnemies%20Spawned (+ (Variables|Default|GetEnemies%20Spawned) 1))
  (AI|SpawnAIFromClass "/Game/Blueprints/Enemy/BP_Enemy_AI.BP_Enemy_AI_C" 0 (Math|Random|RandomPointinBoundingBox (Transformation|GetWorldLocation _spawn_volume) (Components|Box|GetScaledBoxExtent _spawn_volume)) "0, 0, 0" false))

(event EventBeginPlay)

(event Collision|EventActorBeginOverlap
  (params (OtherActor :type Actor%20Object%20Reference)))

(event EventTick
  (params (DeltaSeconds :type Float%20%28single-precision%29))
  ;[1 1 1] Spawns Enemies
  (bind _asbp_game_instance (Utilities|Casting|CastToBP_GameInstance (Game|GetGameInstance)))
  (if (>= (Variables|Default|GetEnemies%20Spawned) (Variables|/Game/Blueprints/BP_GameInstance.BP_GameInstance_C|GetNum%20of%20enemies%20to%20spawn _asbp_game_instance))
    (Variables|Default|SetEnemies%20Spawned 0)
    (Variables|Default|SetMultiple%20Spawns false)
    (Utilities|Time|SetTimerbyEvent (delegate Custom|Numberofenemiesspawned) (Variables|/Game/Blueprints/BP_GameInstance.BP_GameInstance_C|GetEnemy%20Spawn%20Rate (stale Custom|EnemySpawn _asbp_game_instance)) (Variables|Default|GetMultiple%20Spawns))))

(fn ConstructionScript)