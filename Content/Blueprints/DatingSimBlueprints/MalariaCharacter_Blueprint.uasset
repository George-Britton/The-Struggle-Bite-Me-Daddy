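; Dating sim character Blueprint that runs Malaria's dialogue scene, then opens Level_04 at an end-of-scene row.
; Loads DataTable rows into an array at BeginPlay, then PlayLine feeds the dialogue and affection widgets, saving the score to the GameInstance.
; NextLine input advances rows, branching at three choice points through hardcoded row indices and playing reaction sounds.
; Tick swaps the character sprite from each row's Expression.
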(event Custom|EndScene
  ;[1 1 1] Ends the current dialogue scene
  (Widget|RemovefromParent (Variables|Default|GetDisplayDialogueWidget))
  (Variables|Default|SetMalariaScenePlaying false)
  (Game|OpenLevel(byName) "Level_04"))

(event Custom|Play%20Line
  (bind _malariarow (Variables|Default|GetMalariaRow))
  (bind _displaydialoguewidget (Variables|Default|GetDisplayDialogueWidget))
  (bind _arrayofrowsmalaria (Variables|Default|GetArrayOfRowsMalaria))
  (bind _arrayofrowsmalaria_2 (Variables|Default|GetArrayOfRowsMalaria))
  (bind _malariarow_2 (Variables|Default|GetMalariaRow))
  (bind _displaydialoguewidget_2 (Variables|Default|GetDisplayDialogueWidget))
  (bind _displaydialoguewidget_3 (Variables|Default|GetDisplayDialogueWidget))
  (bind _arrayofrowsmalaria_3 (Variables|Default|GetArrayOfRowsMalaria))
  (bind _output (Utilities|Array|Get(acopy) _arrayofrowsmalaria_3 _malariarow))
  (bind _output_2 (Utilities|Array|Get(acopy) _arrayofrowsmalaria_2 _malariarow_2))
  (bind (_speaker _text _expression _options _endscene_ _point) (Utilities|Struct|BreakMalariaDialogueStruct _output_2))
  (bind (_speaker_2 _text_2 _expression_2 _options_2) (Utilities|Struct|BreakMalariaDialogueStruct _output))
  ;[1 1 1] Sets the speaker name and dialogue in the dialogue box
  (if (Utilities|Enum|Equal(Enum) _endscene_ "Yes")
    (CallFunction|EndScene)
    (else
      (Variables|Default|SetRowFinished? false)
      (Variables|Default|SetMalariaScore (+ _point (Variables|Default|GetMalariaScore)))
      (Utilities|IsValid _displaydialoguewidget_2
        (:Is%20Valid
          (Variables|/Game/Blueprints/DatingSimBlueprints/DisplayDialogue.DisplayDialogue_C|SetSpeaker _displaydialoguewidget_2 (Utilities|Text|ToText(String) (Utilities|String|EnumtoString _speaker_2)))
          (Variables|/Game/Blueprints/DatingSimBlueprints/DisplayDialogue.DisplayDialogue_C|SetText _displaydialoguewidget_2 (Utilities|Text|ToText(String) _text_2))
          ;[1 1 1] This FUCKING MESS OF LINGUINE displays the correct dialogue choices when the player needs to choose one
          (if (Utilities|Enum|Equal(Enum) _options_2 "Enabled")
            (Variables|/Game/Blueprints/DatingSimBlueprints/DisplayDialogue.DisplayDialogue_C|SetDialogueArrowSlot _displaydialoguewidget 1)
            (if (== (Variables|Default|GetMalariaChoicesMade) 0)
              (Variables|/Game/Blueprints/DatingSimBlueprints/DisplayDialogue.DisplayDialogue_C|SetChoice1Text _displaydialoguewidget_3 (Utilities|Text|ToText(String) (.Text (Utilities|Struct|BreakMalariaDialogueStruct (Utilities|Array|Get(acopy) _arrayofrowsmalaria 5)))))
              (Variables|/Game/Blueprints/DatingSimBlueprints/DisplayDialogue.DisplayDialogue_C|SetChoice2Text _displaydialoguewidget_3 (Utilities|Text|ToText(String) (.Text (Utilities|Struct|BreakMalariaDialogueStruct (Utilities|Array|Get(acopy) _arrayofrowsmalaria 6)))))
              (bind _output_get (Variables|/Game/Blueprints/Widgets/affectionOverlay.affectionOverlay_C|SetAffectionValue (Variables|Default|GetAffectionOverlayReference) (Variables|Default|GetMalariaScore) :!label _label))
              (bind _asbp_game_instance (Utilities|Casting|CastToBP_GameInstance (Game|GetGameInstance)))
              (Variables|/Game/Blueprints/BP_GameInstance.BP_GameInstance_C|SetMalariaAffScore _asbp_game_instance _output_get)
              (Utilities|FlowControl|Delay 0.2)
              (Variables|Default|SetRowFinished? true)
              (elif (== (Variables|Default|GetMalariaChoicesMade) 1)
                (Variables|/Game/Blueprints/DatingSimBlueprints/DisplayDialogue.DisplayDialogue_C|SetChoice1Text _displaydialoguewidget_3 (Utilities|Text|ToText(String) (.Text (Utilities|Struct|BreakMalariaDialogueStruct (Utilities|Array|Get(acopy) _arrayofrowsmalaria 14)))))
                (Variables|/Game/Blueprints/DatingSimBlueprints/DisplayDialogue.DisplayDialogue_C|SetChoice2Text _displaydialoguewidget_3 (Utilities|Text|ToText(String) (.Text (Utilities|Struct|BreakMalariaDialogueStruct (Utilities|Array|Get(acopy) _arrayofrowsmalaria 15)))))
                (goto _label)
                (elif (== (Variables|Default|GetMalariaChoicesMade) 2)
                  (Variables|/Game/Blueprints/DatingSimBlueprints/DisplayDialogue.DisplayDialogue_C|SetChoice1Text _displaydialoguewidget_3 (Utilities|Text|ToText(String) (.Text (Utilities|Struct|BreakMalariaDialogueStruct (Utilities|Array|Get(acopy) _arrayofrowsmalaria 28)))))
                  (Variables|/Game/Blueprints/DatingSimBlueprints/DisplayDialogue.DisplayDialogue_C|SetChoice2Text _displaydialoguewidget_3 (Utilities|Text|ToText(String) (.Text (Utilities|Struct|BreakMalariaDialogueStruct (Utilities|Array|Get(acopy) _arrayofrowsmalaria 29)))))
                  (goto _label))))
            (else
              (Variables|/Game/Blueprints/DatingSimBlueprints/DisplayDialogue.DisplayDialogue_C|SetDialogueArrowSlot _displaydialoguewidget 3)
              (Variables|/Game/Blueprints/DatingSimBlueprints/DisplayDialogue.DisplayDialogue_C|SetChoice1Text _displaydialoguewidget "        ")
              (Variables|/Game/Blueprints/DatingSimBlueprints/DisplayDialogue.DisplayDialogue_C|SetChoice2Text _displaydialoguewidget "            ")
              (goto _label))))))))

(event Custom|InitiateMalriaScene
  (params (NewParam :type Data%20Table%20Object%20Reference))
  ;[1 1 1] Gets the data from the Speaker and Text rows of the dialogue file
  (bind _outrownames (DataTable|GetDataTableRowNames "/Game/Assets/Dialogue/Malaria/MalariaDialogue.MalariaDialogue"))
  (for _array_element _outrownames
    (bind _returnvalue (Utilities|GetDataTableRow "/Game/Assets/Dialogue/Malaria/MalariaDialogue.MalariaDialogue" _array_element)
      (:then
        (Utilities|Array|Add (Variables|Default|GetArrayOfRowsMalaria) _returnvalue))))
  (bind _returnvalue_2 (UserInterface|CreateWidget "/Game/Blueprints/DatingSimBlueprints/DisplayDialogue.DisplayDialogue_C"))
  (bind _output_get (Variables|Default|SetDisplayDialogueWidget _returnvalue_2))
  (UserInterface|Viewport|AddtoViewport _output_get 0)
  (bind _returnvalue_3 (UserInterface|CreateWidget "/Game/Blueprints/Widgets/affectionOverlay.affectionOverlay_C"))
  (bind _output_get_2 (Variables|Default|SetAffectionOverlayReference _returnvalue_3))
  (UserInterface|Viewport|AddtoViewport _output_get_2 0)
  (CallFunction|PlayLine))

(event EventBeginPlay
  ;[1 1 1] Starts the scene and enables input
  (if (not (Variables|Default|GetMalariaScenePlaying))
    (Variables|Default|SetMalariaScenePlaying false)
    (CallFunction|InitiateMalriaScene "/Game/Assets/Dialogue/Malaria/MalariaDialogue.MalariaDialogue")
    (Input|EnableInput (Game|GetPlayerController 0))))

(event EventTick
  (params (DeltaSeconds :type Float%20%28single-precision%29))
  (bind _arrayofrowsmalaria (Variables|Default|GetArrayOfRowsMalaria))
  (bind _malariarow (Variables|Default|GetMalariaRow))
  (bind _output (Utilities|Array|Get(acopy) _arrayofrowsmalaria _malariarow))
  (bind _expression (Utilities|Struct|BreakMalariaDialogueStruct _output))
  ;[1 1 1] Changes the character's facial expression
  (if (Utilities|Enum|Equal(Enum) _expression "Neutral")
    (Rendering|Components|Sprite|SetSprite (Variables|Default|GetMalariaSprite) "/Game/Assets/Images/Malaria/MalariaNeutral_Sprite.MalariaNeutral_Sprite")
    (elif (Utilities|Enum|Equal(Enum) _expression "Angry")
      (Rendering|Components|Sprite|SetSprite (Variables|Default|GetMalariaSprite) "/Game/Assets/Images/Malaria/MalariaAngry_Sprite.MalariaAngry_Sprite")
      (elif (Utilities|Enum|Equal(Enum) _expression "Happy")
        (Rendering|Components|Sprite|SetSprite (Variables|Default|GetMalariaSprite) "/Game/Assets/Images/Malaria/MalariaHappy_Sprite.MalariaHappy_Sprite")))))

(event Input|ActionEvents|InputActionNextLine
  (params (Key :type Key%20Structure))
  (bind _displaydialoguewidget (Variables|Default|GetDisplayDialogueWidget))
  (bind _dialoguearrowslot (Variables|/Game/Blueprints/DatingSimBlueprints/DisplayDialogue.DisplayDialogue_C|GetDialogueArrowSlot _displaydialoguewidget))
  (bind _returnvalue (== _dialoguearrowslot 1))
  ;[1 1 1] Progresses the dialogue
  (:Pressed
    (if (Variables|Default|GetRowFinished?)
      (if (Utilities|Enum|Equal(Enum) (.Options (Utilities|Struct|BreakMalariaDialogueStruct (Utilities|Array|Get(acopy) (Variables|Default|GetArrayOfRowsMalaria) (Variables|Default|GetMalariaRow)))) "Disabled")
        (Variables|Default|SetMalariaRow (+ (Variables|Default|GetMalariaRow) 1))
        (else
          (if (== (Variables|Default|GetMalariaChoicesMade) 0)
            (if _returnvalue
              (Variables|Default|SetMalariaRow 8)
              (Audio|PlaySound2D "/Game/Assets/Sound/MalariaAngrySound.MalariaAngrySound" :!label _label)
              (else
                (Variables|Default|SetMalariaRow 11)
                (Audio|PlaySound2D "/Game/Assets/Sound/MalariaLaughSound.MalariaLaughSound" :!label _label_2)))
            (elif (== (Variables|Default|GetMalariaChoicesMade) 1)
              (if _returnvalue
                (Variables|Default|SetMalariaRow 17)
                (goto _label)
                (else
                  (Variables|Default|SetMalariaRow 21)
                  (goto _label_2)))
              (elif _returnvalue
                (Variables|Default|SetMalariaRow 31)
                (goto _label_2)
                (else
                  (Variables|Default|SetMalariaRow 34)
                  (goto _label)))))
          (Variables|Default|SetMalariaChoicesMade (+ (Variables|Default|GetMalariaChoicesMade) 1))))
      (CallFunction|PlayLine))))

(event Input|ActionEvents|InputActionSelectUp
  (params (Key :type Key%20Structure))
  (bind _displaydialoguewidget (Variables|Default|GetDisplayDialogueWidget))
  ;[1 1 1] Sets the location for the dialogue arrow
  (:Pressed
    (if (Utilities|Enum|Equal(Enum) (.Options (Utilities|Struct|BreakMalariaDialogueStruct (Utilities|Array|Get(acopy) (Variables|Default|GetArrayOfRowsMalaria) (Variables|Default|GetMalariaRow)))) "Enabled")
      (Variables|/Game/Blueprints/DatingSimBlueprints/DisplayDialogue.DisplayDialogue_C|SetDialogueArrowSlot _displaydialoguewidget 1)
      (else
        (Variables|/Game/Blueprints/DatingSimBlueprints/DisplayDialogue.DisplayDialogue_C|SetDialogueArrowSlot _displaydialoguewidget 3)))))

(event Input|ActionEvents|InputActionSelectDown
  (params (Key :type Key%20Structure))
  (bind _displaydialoguewidget (Variables|Default|GetDisplayDialogueWidget))
  ;[1 1 1] Sets the location for the dialogue arrow
  (:Pressed
    (if (Utilities|Enum|Equal(Enum) (.Options (Utilities|Struct|BreakMalariaDialogueStruct (Utilities|Array|Get(acopy) (Variables|Default|GetArrayOfRowsMalaria) (Variables|Default|GetMalariaRow)))) "Enabled")
      (Variables|/Game/Blueprints/DatingSimBlueprints/DisplayDialogue.DisplayDialogue_C|SetDialogueArrowSlot _displaydialoguewidget 2)
      (else
        (Variables|/Game/Blueprints/DatingSimBlueprints/DisplayDialogue.DisplayDialogue_C|SetDialogueArrowSlot _displaydialoguewidget 3)))))

(fn ConstructionScript)