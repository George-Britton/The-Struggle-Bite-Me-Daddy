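; Bona Lisa's dating-sim character, which runs their dialogue scene and opens Level_02 when it ends.
; BeginPlay loads BonaDialogue data table rows into an array and creates dialogue and affection widgets; Tick sets the expression sprite from the current row.
; Input advances lines or picks between two options, branching through hard-coded row indices keyed on choices made.
; PlayLine fills the dialogue box and accumulates row points into the overlay and GameInstance affection score.
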(event Custom|InitiateBonaLisaScene
  (params (BonaLisaScene :type Data%20Table%20Object%20Reference))
  ;[1 1 1] Gets the data from the Speaker and Text rows of the dialogue file
  (bind _outrownames (DataTable|GetDataTableRowNames "/Game/Assets/Dialogue/BonaLisa/BonaDialogue.BonaDialogue"))
  (for _array_element _outrownames
    (bind _returnvalue (Utilities|GetDataTableRow "/Game/Assets/Dialogue/BonaLisa/BonaDialogue.BonaDialogue" _array_element)
      (:then
        (Utilities|Array|Add (Variables|Default|GetArrayofRowsBonaLisa) _returnvalue))))
  (bind _returnvalue_2 (UserInterface|CreateWidget "/Game/Blueprints/DatingSimBlueprints/DisplayDialogue.DisplayDialogue_C"))
  (bind _output_get (Variables|Default|SetDisplayDialogueWidget _returnvalue_2))
  (UserInterface|Viewport|AddtoViewport _output_get 0)
  (bind _returnvalue_3 (UserInterface|CreateWidget "/Game/Blueprints/Widgets/affectionOverlay.affectionOverlay_C"))
  (bind _output_get_2 (Variables|Default|SetAffectionOverlayReference _returnvalue_3))
  (UserInterface|Viewport|AddtoViewport _output_get_2 0)
  (CallFunction|PlayLine))

(event Custom|Play%20Line
  (bind _bonalisarow (Variables|Default|GetBonaLisaRow))
  (bind _arrayofrowsbonalisa (Variables|Default|GetArrayofRowsBonaLisa))
  (bind _arrayofrowsbonalisa_2 (Variables|Default|GetArrayofRowsBonaLisa))
  (bind _arrayofrowsbonalisa_3 (Variables|Default|GetArrayofRowsBonaLisa))
  (bind _displaydialoguewidget (Variables|Default|GetDisplayDialogueWidget))
  (bind _bonalisarow_2 (Variables|Default|GetBonaLisaRow))
  (bind _displaydialoguewidget_2 (Variables|Default|GetDisplayDialogueWidget))
  (bind _displaydialoguewidget_3 (Variables|Default|GetDisplayDialogueWidget))
  (bind _output (Utilities|Array|Get(acopy) _arrayofrowsbonalisa _bonalisarow))
  (bind _output_2 (Utilities|Array|Get(acopy) _arrayofrowsbonalisa_2 _bonalisarow_2))
  (bind (_speaker _text _expression _options) (Utilities|Struct|BreakBonaDialogueStruct _output_2))
  (bind (_speaker_2 _text_2 _expression_2 _options_2 _endscene_ _point) (Utilities|Struct|BreakBonaDialogueStruct _output))
  ;[1 1 1] Sets the speaker name and dialogue in the dialogue box
  (if (Utilities|Enum|Equal(Enum) _endscene_ "Yes")
    (CallFunction|EndScene)
    (else
      (Variables|Default|SetRowFinished? false)
      (Variables|Default|SetBonaLisaScore (+ _point (Variables|Default|GetBonaLisaScore)))
      (Utilities|IsValid _displaydialoguewidget_2
        (:Is%20Valid
          (Variables|/Game/Blueprints/DatingSimBlueprints/DisplayDialogue.DisplayDialogue_C|SetSpeaker _displaydialoguewidget_2 (Utilities|Text|ToText(String) (Utilities|String|EnumtoString _speaker)))
          (Variables|/Game/Blueprints/DatingSimBlueprints/DisplayDialogue.DisplayDialogue_C|SetText _displaydialoguewidget_2 (Utilities|Text|ToText(String) _text))
          ;[1 1 1] This FUCKING MESS OF LINGUINE displays the correct dialogue choices when the player needs to choose one
          (if (Utilities|Enum|Equal(Enum) _options "Enabled")
            (Variables|/Game/Blueprints/DatingSimBlueprints/DisplayDialogue.DisplayDialogue_C|SetDialogueArrowSlot _displaydialoguewidget 1)
            (if (== (Variables|Default|GetBonaLisaChoicesMade) 0)
              (Variables|/Game/Blueprints/DatingSimBlueprints/DisplayDialogue.DisplayDialogue_C|SetChoice1Text _displaydialoguewidget (Utilities|Text|ToText(String) (.Text (Utilities|Struct|BreakBonaDialogueStruct (Utilities|Array|Get(acopy) _arrayofrowsbonalisa_3 6)))))
              (Variables|/Game/Blueprints/DatingSimBlueprints/DisplayDialogue.DisplayDialogue_C|SetChoice2Text _displaydialoguewidget (Utilities|Text|ToText(String) (.Text (Utilities|Struct|BreakBonaDialogueStruct (Utilities|Array|Get(acopy) _arrayofrowsbonalisa_3 7)))))
              (bind _output_get (Variables|/Game/Blueprints/Widgets/affectionOverlay.affectionOverlay_C|SetAffectionValue (Variables|Default|GetAffectionOverlayReference) (Variables|Default|GetBonaLisaScore) :!label _label))
              (bind _asbp_game_instance (Utilities|Casting|CastToBP_GameInstance (Game|GetGameInstance)))
              (Variables|/Game/Blueprints/BP_GameInstance.BP_GameInstance_C|SetBonaLisaAffScore _asbp_game_instance _output_get)
              (Utilities|FlowControl|Delay 0.2)
              (Variables|Default|SetRowFinished? true)
              (elif (== (Variables|Default|GetBonaLisaChoicesMade) 1)
                (Variables|/Game/Blueprints/DatingSimBlueprints/DisplayDialogue.DisplayDialogue_C|SetChoice1Text _displaydialoguewidget_3 (Utilities|Text|ToText(String) (.Text (Utilities|Struct|BreakBonaDialogueStruct (Utilities|Array|Get(acopy) _arrayofrowsbonalisa_3 15)))))
                (Variables|/Game/Blueprints/DatingSimBlueprints/DisplayDialogue.DisplayDialogue_C|SetChoice2Text _displaydialoguewidget_3 (Utilities|Text|ToText(String) (.Text (Utilities|Struct|BreakBonaDialogueStruct (Utilities|Array|Get(acopy) _arrayofrowsbonalisa_3 16)))))
                (goto _label)
                (elif (== (Variables|Default|GetBonaLisaChoicesMade) 2)
                  (Variables|/Game/Blueprints/DatingSimBlueprints/DisplayDialogue.DisplayDialogue_C|SetChoice1Text _displaydialoguewidget_3 (Utilities|Text|ToText(String) (.Text (Utilities|Struct|BreakBonaDialogueStruct (Utilities|Array|Get(acopy) _arrayofrowsbonalisa_3 27)))))
                  (Variables|/Game/Blueprints/DatingSimBlueprints/DisplayDialogue.DisplayDialogue_C|SetChoice2Text _displaydialoguewidget_3 (Utilities|Text|ToText(String) (.Text (Utilities|Struct|BreakBonaDialogueStruct (Utilities|Array|Get(acopy) _arrayofrowsbonalisa_3 28)))))
                  (goto _label))))
            (else
              (Variables|/Game/Blueprints/DatingSimBlueprints/DisplayDialogue.DisplayDialogue_C|SetDialogueArrowSlot _displaydialoguewidget 3)
              (Variables|/Game/Blueprints/DatingSimBlueprints/DisplayDialogue.DisplayDialogue_C|SetChoice1Text _displaydialoguewidget "        ")
              (Variables|/Game/Blueprints/DatingSimBlueprints/DisplayDialogue.DisplayDialogue_C|SetChoice2Text _displaydialoguewidget "            ")
              (goto _label))))))))

(event Custom|EndScene
  ;[1 1 1] Ends the current dialogue scene
  (Widget|RemovefromParent (Variables|Default|GetDisplayDialogueWidget))
  (Variables|Default|SetBonaLisaScenePlaying false)
  (Game|OpenLevel(byName) "Level_02"))

(event EventBeginPlay
  ;[1 1 1] Starts the scene and enables input
  (if (not (Variables|Default|GetBonaLisaScenePlaying))
    (Variables|Default|SetBonaLisaScenePlaying false)
    (CallFunction|InitiateBonaLisaScene "/Game/Assets/Dialogue/BonaLisa/BonaDialogue.BonaDialogue")
    (Input|EnableInput (Game|GetPlayerController 0))))

(event EventTick
  (params (DeltaSeconds :type Float%20%28single-precision%29))
  (bind _arrayofrowsbonalisa (Variables|Default|GetArrayofRowsBonaLisa))
  (bind _bonalisarow (Variables|Default|GetBonaLisaRow))
  (bind _output (Utilities|Array|Get(acopy) _arrayofrowsbonalisa _bonalisarow))
  (bind _expression (Utilities|Struct|BreakBonaDialogueStruct _output))
  ;[1 1 1] Changes the character's facial expression
  (if (Utilities|Enum|Equal(Enum) _expression "Neutral")
    (Rendering|Components|Sprite|SetSprite (Variables|Default|GetBonaLisaSprite) "/Game/Assets/Images/BonaLisa/BonaLisaNeutral_Sprite.BonaLisaNeutral_Sprite")
    (elif (Utilities|Enum|Equal(Enum) _expression "Angry")
      (Rendering|Components|Sprite|SetSprite (Variables|Default|GetBonaLisaSprite) "/Game/Assets/Images/BonaLisa/BonaLisaAngry_Sprite.BonaLisaAngry_Sprite")
      (elif (Utilities|Enum|Equal(Enum) _expression "Happy")
        (Rendering|Components|Sprite|SetSprite (Variables|Default|GetBonaLisaSprite) "/Game/Assets/Images/BonaLisa/BonaLisaHappy_Sprite.BonaLisaHappy_Sprite")))))

(event Input|ActionEvents|InputActionNextLine
  (params (Key :type Key%20Structure))
  (bind _displaydialoguewidget (Variables|Default|GetDisplayDialogueWidget))
  (bind _dialoguearrowslot (Variables|/Game/Blueprints/DatingSimBlueprints/DisplayDialogue.DisplayDialogue_C|GetDialogueArrowSlot _displaydialoguewidget))
  (bind _returnvalue (== _dialoguearrowslot 1))
  ;[1 1 1] Progresses the dialogue
  (:Pressed
    (if (Variables|Default|GetRowFinished?)
      (if (Utilities|Enum|Equal(Enum) (.Options (Utilities|Struct|BreakBonaDialogueStruct (Utilities|Array|Get(acopy) (Variables|Default|GetArrayofRowsBonaLisa) (Variables|Default|GetBonaLisaRow)))) "Disabled")
        (Variables|Default|SetBonaLisaRow (+ (Variables|Default|GetBonaLisaRow) 1))
        (else
          (if (== (Variables|Default|GetBonaLisaChoicesMade) 0)
            (if _returnvalue
              (Variables|Default|SetBonaLisaRow 9)
              (Audio|PlaySound2D "/Game/Assets/Sound/BonaLisaAngrySound.BonaLisaAngrySound" :!label _label)
              (else
                (Variables|Default|SetBonaLisaRow 12)
                (Audio|PlaySound2D "/Game/Assets/Sound/BonaLisaLaughSound.BonaLisaLaughSound" :!label _label_2)))
            (elif (== (Variables|Default|GetBonaLisaChoicesMade) 1)
              (if _returnvalue
                (Variables|Default|SetBonaLisaRow 21)
                (goto _label_2)
                (else
                  (Variables|Default|SetBonaLisaRow 18)
                  (goto _label)))
              (elif _returnvalue
                (Variables|Default|SetBonaLisaRow 30)
                (goto _label)
                (else
                  (Variables|Default|SetBonaLisaRow 33)
                  (goto _label_2)))))
          (Variables|Default|SetBonaLisaChoicesMade (+ (Variables|Default|GetBonaLisaChoicesMade) 1))))
      (CallFunction|PlayLine))))

(event Input|ActionEvents|InputActionSelectUp
  (params (Key :type Key%20Structure))
  (bind _displaydialoguewidget (Variables|Default|GetDisplayDialogueWidget))
  ;[1 1 1] Sets the location for the dialogue arrow
  (:Pressed
    (if (Utilities|Enum|Equal(Enum) (.Options (Utilities|Struct|BreakBonaDialogueStruct (Utilities|Array|Get(acopy) (Variables|Default|GetArrayofRowsBonaLisa) (Variables|Default|GetBonaLisaRow)))) "Enabled")
      (Variables|/Game/Blueprints/DatingSimBlueprints/DisplayDialogue.DisplayDialogue_C|SetDialogueArrowSlot _displaydialoguewidget 1)
      (else
        (Variables|/Game/Blueprints/DatingSimBlueprints/DisplayDialogue.DisplayDialogue_C|SetDialogueArrowSlot _displaydialoguewidget 3)))))

(event Input|ActionEvents|InputActionSelectDown
  (params (Key :type Key%20Structure))
  (bind _displaydialoguewidget (Variables|Default|GetDisplayDialogueWidget))
  ;[1 1 1] Sets the location for the dialogue arrow
  (:Pressed
    (if (Utilities|Enum|Equal(Enum) (.Options (Utilities|Struct|BreakBonaDialogueStruct (Utilities|Array|Get(acopy) (Variables|Default|GetArrayofRowsBonaLisa) (Variables|Default|GetBonaLisaRow)))) "Enabled")
      (Variables|/Game/Blueprints/DatingSimBlueprints/DisplayDialogue.DisplayDialogue_C|SetDialogueArrowSlot _displaydialoguewidget 2)
      (else
        (Variables|/Game/Blueprints/DatingSimBlueprints/DisplayDialogue.DisplayDialogue_C|SetDialogueArrowSlot _displaydialoguewidget 3)))))

(fn ConstructionScript)