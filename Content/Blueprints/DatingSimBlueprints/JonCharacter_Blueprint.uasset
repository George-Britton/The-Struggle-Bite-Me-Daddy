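; Dating-sim character Blueprint for Jon that runs his dialogue scene, then opens Level_03 when it ends.
; BeginPlay loads dialogue DataTable rows into an array and creates dialogue and affection widgets.
; NextLine advances rows or branches at three two-option choices using hard-coded indices, with arrow selection and reaction sounds.
; PlayLine fills the dialogue box and accumulates affection into the game instance, while Tick swaps expression sprites from the current row.
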(event Custom|EndScene
  ;[1 1 1] Ends the current dialogue scene
  (Widget|RemovefromParent (Variables|Default|GetDisplayDialogueWidget))
  (Variables|Default|SetJonScenePlaying false)
  (Game|OpenLevel(byName) "Level_03"))

(event Custom|Play%20Line
  (bind _arrayofrowsjon (Variables|Default|GetArrayOfRowsJon))
  (bind _arrayofrowsjon_2 (Variables|Default|GetArrayOfRowsJon))
  (bind _jonrow (Variables|Default|GetJonRow))
  (bind _displaydialoguewidget (Variables|Default|GetDisplayDialogueWidget))
  (bind _displaydialoguewidget_2 (Variables|Default|GetDisplayDialogueWidget))
  (bind _displaydialoguewidget_3 (Variables|Default|GetDisplayDialogueWidget))
  (bind _arrayofrowsjon_3 (Variables|Default|GetArrayOfRowsJon))
  (bind _jonrow_2 (Variables|Default|GetJonRow))
  (bind _output (Utilities|Array|Get(acopy) _arrayofrowsjon_3 _jonrow_2))
  (bind _output_2 (Utilities|Array|Get(acopy) _arrayofrowsjon_2 _jonrow))
  (bind (_speaker _text _expression _options) (Utilities|Struct|BreakJonDialogueStruct _output_2))
  (bind (_speaker_2 _text_2 _expression_2 _options_2 _endscene_ _point) (Utilities|Struct|BreakJonDialogueStruct _output))
  ;[1 1 1] Sets the speaker name and dialogue in the dialogue box
  (if (Utilities|Enum|Equal(Enum) _endscene_ "Yes")
    (CallFunction|EndScene)
    (else
      (Variables|Default|SetRowFinished? false)
      (Variables|Default|SetJonScore (+ _point (Variables|Default|GetJonScore)))
      (Utilities|IsValid _displaydialoguewidget_2
        (:Is%20Valid
          (Variables|/Game/Blueprints/DatingSimBlueprints/DisplayDialogue.DisplayDialogue_C|SetSpeaker _displaydialoguewidget_2 (Utilities|Text|ToText(String) (Utilities|String|EnumtoString _speaker)))
          (Variables|/Game/Blueprints/DatingSimBlueprints/DisplayDialogue.DisplayDialogue_C|SetText _displaydialoguewidget_2 (Utilities|Text|ToText(String) _text))
          ;[1 1 1] This FUCKING MESS OF LINGUINE displays the correct dialogue choices when the player needs to choose one
          (if (Utilities|Enum|Equal(Enum) _options "Enabled")
            (Variables|/Game/Blueprints/DatingSimBlueprints/DisplayDialogue.DisplayDialogue_C|SetDialogueArrowSlot _displaydialoguewidget 1)
            (if (== (Variables|Default|GetJonChoicesMade) 0)
              (Variables|/Game/Blueprints/DatingSimBlueprints/DisplayDialogue.DisplayDialogue_C|SetChoice1Text _displaydialoguewidget (Utilities|Text|ToText(String) (.Text (Utilities|Struct|BreakJonDialogueStruct (Utilities|Array|Get(acopy) _arrayofrowsjon 6)))))
              (Variables|/Game/Blueprints/DatingSimBlueprints/DisplayDialogue.DisplayDialogue_C|SetChoice2Text _displaydialoguewidget (Utilities|Text|ToText(String) (.Text (Utilities|Struct|BreakJonDialogueStruct (Utilities|Array|Get(acopy) _arrayofrowsjon 7)))))
              (bind _output_get (Variables|/Game/Blueprints/Widgets/affectionOverlay.affectionOverlay_C|SetAffectionValue (Variables|Default|GetAffectionOverlayReferemce) (Variables|Default|GetJonScore) :!label _label))
              (bind _asbp_game_instance (Utilities|Casting|CastToBP_GameInstance (Game|GetGameInstance)))
              (Variables|/Game/Blueprints/BP_GameInstance.BP_GameInstance_C|SetJonAffScore _asbp_game_instance _output_get)
              (Utilities|FlowControl|Delay 0.2)
              (Variables|Default|SetRowFinished? true)
              (elif (== (Variables|Default|GetJonChoicesMade) 1)
                (Variables|/Game/Blueprints/DatingSimBlueprints/DisplayDialogue.DisplayDialogue_C|SetChoice1Text _displaydialoguewidget_3 (Utilities|Text|ToText(String) (.Text (Utilities|Struct|BreakJonDialogueStruct (Utilities|Array|Get(acopy) _arrayofrowsjon 15)))))
                (Variables|/Game/Blueprints/DatingSimBlueprints/DisplayDialogue.DisplayDialogue_C|SetChoice2Text _displaydialoguewidget_3 (Utilities|Text|ToText(String) (.Text (Utilities|Struct|BreakJonDialogueStruct (Utilities|Array|Get(acopy) _arrayofrowsjon 16)))))
                (goto _label)
                (elif (== (Variables|Default|GetJonChoicesMade) 2)
                  (Variables|/Game/Blueprints/DatingSimBlueprints/DisplayDialogue.DisplayDialogue_C|SetChoice1Text _displaydialoguewidget_3 (Utilities|Text|ToText(String) (.Text (Utilities|Struct|BreakJonDialogueStruct (Utilities|Array|Get(acopy) _arrayofrowsjon 27)))))
                  (Variables|/Game/Blueprints/DatingSimBlueprints/DisplayDialogue.DisplayDialogue_C|SetChoice2Text _displaydialoguewidget_3 (Utilities|Text|ToText(String) (.Text (Utilities|Struct|BreakJonDialogueStruct (Utilities|Array|Get(acopy) _arrayofrowsjon 28)))))
                  (goto _label))))
            (else
              (Variables|/Game/Blueprints/DatingSimBlueprints/DisplayDialogue.DisplayDialogue_C|SetDialogueArrowSlot _displaydialoguewidget 3)
              (Variables|/Game/Blueprints/DatingSimBlueprints/DisplayDialogue.DisplayDialogue_C|SetChoice1Text _displaydialoguewidget "        ")
              (Variables|/Game/Blueprints/DatingSimBlueprints/DisplayDialogue.DisplayDialogue_C|SetChoice2Text _displaydialoguewidget "            ")
              (goto _label))))))))

(event Custom|InitiateJonScene
  (params (JonScene :type Data%20Table%20Object%20Reference))
  ;[1 1 1] Gets the data from the Speaker and Text rows of the dialogue file
  (bind _outrownames (DataTable|GetDataTableRowNames "/Game/Assets/Dialogue/JonBoneJovi/JonDialogue.JonDialogue"))
  (for _array_element _outrownames
    (bind _returnvalue (Utilities|GetDataTableRow "/Game/Assets/Dialogue/JonBoneJovi/JonDialogue.JonDialogue" _array_element)
      (:then
        (Utilities|Array|Add (Variables|Default|GetArrayOfRowsJon) _returnvalue))))
  (bind _returnvalue_2 (UserInterface|CreateWidget "/Game/Blueprints/DatingSimBlueprints/DisplayDialogue.DisplayDialogue_C"))
  (bind _output_get (Variables|Default|SetDisplayDialogueWidget _returnvalue_2))
  (UserInterface|Viewport|AddtoViewport _output_get 0)
  (bind _returnvalue_3 (UserInterface|CreateWidget "/Game/Blueprints/Widgets/affectionOverlay.affectionOverlay_C"))
  (bind _output_get_2 (Variables|Default|SetAffectionOverlayReferemce _returnvalue_3))
  (UserInterface|Viewport|AddtoViewport _output_get_2 0)
  (CallFunction|PlayLine))

(event EventBeginPlay
  ;[1 1 1] Starts the scene and enables input
  (if (not (Variables|Default|GetJonScenePlaying))
    (Variables|Default|SetJonScenePlaying false)
    (CallFunction|InitiateJonScene)
    (Input|EnableInput (Game|GetPlayerController 0))))

(event EventTick
  (params (DeltaSeconds :type Float%20%28single-precision%29))
  (bind _jonrow (Variables|Default|GetJonRow))
  (bind _arrayofrowsjon (Variables|Default|GetArrayOfRowsJon))
  (bind _output (Utilities|Array|Get(acopy) _arrayofrowsjon _jonrow))
  (bind _expression (Utilities|Struct|BreakJonDialogueStruct _output))
  ;[1 1 1] Changes the character's facial expression
  (if (Utilities|Enum|Equal(Enum) _expression "Neutral")
    (Rendering|Components|Sprite|SetSprite (Variables|Default|GetJonSprite) "/Game/Assets/Images/JonBoneJovi/JonNeutral_Sprite.JonNeutral_Sprite")
    (elif (Utilities|Enum|Equal(Enum) _expression "Angry")
      (Rendering|Components|Sprite|SetSprite (Variables|Default|GetJonSprite) "/Game/Assets/Images/JonBoneJovi/JonAngry_Sprite.JonAngry_Sprite")
      (elif (Utilities|Enum|Equal(Enum) _expression "Happy")
        (Rendering|Components|Sprite|SetSprite (Variables|Default|GetJonSprite) "/Game/Assets/Images/JonBoneJovi/JonHappy_Sprite.JonHappy_Sprite")))))

(event Input|ActionEvents|InputActionNextLine
  (params (Key :type Key%20Structure))
  (bind _displaydialoguewidget (Variables|Default|GetDisplayDialogueWidget))
  (bind _dialoguearrowslot (Variables|/Game/Blueprints/DatingSimBlueprints/DisplayDialogue.DisplayDialogue_C|GetDialogueArrowSlot _displaydialoguewidget))
  (bind _returnvalue (== _dialoguearrowslot 1))
  ;[1 1 1] Progresses the dialogue
  (:Pressed
    (if (Variables|Default|GetRowFinished?)
      (if (Utilities|Enum|Equal(Enum) (.Options (Utilities|Struct|BreakJonDialogueStruct (Utilities|Array|Get(acopy) (Variables|Default|GetArrayOfRowsJon) (Variables|Default|GetJonRow)))) "Disabled")
        (Variables|Default|SetJonRow (+ (Variables|Default|GetJonRow) 1))
        (else
          (if (== (Variables|Default|GetJonChoicesMade) 0)
            (if _returnvalue
              (Variables|Default|SetJonRow 9)
              (Audio|PlaySound2D "/Game/Assets/Sound/JonBoneJoviAngrySound.JonBoneJoviAngrySound" :!label _label)
              (else
                (Variables|Default|SetJonRow 12)
                (Audio|PlaySound2D "/Game/Assets/Sound/JonBoneJoviLaughSound.JonBoneJoviLaughSound" :!label _label_2)))
            (elif (== (Variables|Default|GetJonChoicesMade) 1)
              (if _returnvalue
                (Variables|Default|SetJonRow 18)
                (goto _label)
                (else
                  (Variables|Default|SetJonRow 22)
                  (goto _label_2)))
              (elif _returnvalue
                (Variables|Default|SetJonRow 30)
                (goto _label)
                (else
                  (Variables|Default|SetJonRow 36)
                  (goto _label_2)))))
          (Variables|Default|SetJonChoicesMade (+ (Variables|Default|GetJonChoicesMade) 1))))
      (CallFunction|PlayLine))))

(event Input|ActionEvents|InputActionSelectUp
  (params (Key :type Key%20Structure))
  (bind _displaydialoguewidget (Variables|Default|GetDisplayDialogueWidget))
  ;[1 1 1] Sets the location for the dialogue arrow
  (:Pressed
    (if (Utilities|Enum|Equal(Enum) (.Options (Utilities|Struct|BreakJonDialogueStruct (Utilities|Array|Get(acopy) (Variables|Default|GetArrayOfRowsJon) (Variables|Default|GetJonRow)))) "Enabled")
      (Variables|/Game/Blueprints/DatingSimBlueprints/DisplayDialogue.DisplayDialogue_C|SetDialogueArrowSlot _displaydialoguewidget 1)
      (else
        (Variables|/Game/Blueprints/DatingSimBlueprints/DisplayDialogue.DisplayDialogue_C|SetDialogueArrowSlot _displaydialoguewidget 3)))))

(event Input|ActionEvents|InputActionSelectDown
  (params (Key :type Key%20Structure))
  (bind _displaydialoguewidget (Variables|Default|GetDisplayDialogueWidget))
  ;[1 1 1] Sets the location for the dialogue arrow
  (:Pressed
    (if (Utilities|Enum|Equal(Enum) (.Options (Utilities|Struct|BreakJonDialogueStruct (Utilities|Array|Get(acopy) (Variables|Default|GetArrayOfRowsJon) (Variables|Default|GetJonRow)))) "Enabled")
      (Variables|/Game/Blueprints/DatingSimBlueprints/DisplayDialogue.DisplayDialogue_C|SetDialogueArrowSlot _displaydialoguewidget 2)
      (else
        (Variables|/Game/Blueprints/DatingSimBlueprints/DisplayDialogue.DisplayDialogue_C|SetDialogueArrowSlot _displaydialoguewidget 3)))))

(fn ConstructionScript)